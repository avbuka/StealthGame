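; Guard character that shows its alert state (idle, suspicious or alerted) as a symbol in a widget.
; On a state change, it updates the WBP_GuardState text and immediately stops its movement.
; The construction script collects every TargetPoint in the level, but the AIMoveTo loop meant to visit five of them is unconnected and never runs.
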(event `self.ReceiveBeginPlay`)

(event `self.OnStateChanged`
  (params (NewState :type "EAIState Enum" :default "Idle"))
  (bind _aswbp_guard_state (cast `/Game/UI/WBP_GuardState` (`WidgetComponent.GetUserWidgetObject` (`self.GuardStateWidget`))))
  (`/Game/UI/WBP_GuardState.UpdateText` _aswbp_guard_state (select `EAIState` NewState :`Suspicious` "?" :`Alerted` "!" :!type "Text"))
  (`MovementComponent.StopMovementImmediately` (`self.CharacterMovement`)))

(fn `UserConstructionScript`
  (bind _outactors (`GameplayStatics.GetAllActorsOfClass` "/Script/Engine.TargetPoint"))
  (set `self.ArrayOfTargets` _outactors))